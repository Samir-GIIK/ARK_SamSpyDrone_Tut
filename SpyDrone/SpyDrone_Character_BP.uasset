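; Flying spy drone character that a player pilots, with Q handing possession back to the stored player pawn.
; Multicast activate/deactivate events switch flying or falling movement and toggle thrusters, sound and material, with deactivation also ejecting the pilot.
; Non-dedicated timer updates bank the mesh from velocity and turn rate and play rotor turn montages.
; Damage drives a health-based particle parameter; on death it falls, polling ground traces before applying a dissolve buff.
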(event `self.ReceiveBeginPlay`
  ;[0.214 1 0.3021] Begin play
  (`parent.ReceiveBeginPlay`)
  (`self.UpdateDamageEffect`)
  (add `self.OnDied` (delegate `OnDied_Event`)))

(event `OnDied_Event` :!signature `self.OnDied`
  (params (DiedCharacter :type "PrimalCharacter Object Reference"))
  ;[0.245 0.1192 0.06448] Died event
  (`self.Multi_DeathUpdateParticles`)
  (`self.SetTickFunctionEnabled` false)
  (`self.BPNetSetCharacterMovementVelocity` false (0.0 0.0 0.0) true "MOVE_Falling")
  (`KismetSystemLibrary.K2_SetTimer` null "DestroySelf" 0.15))

(event `Multi_DeathUpdateParticles`
  ;[0.61 0.02531 0] Update particles on death
  (`ActorComponent.Deactivate` (`self.DamageEffect`))
  (`ActorComponent.Deactivate` (`self.WingThrusterL`))
  (`ActorComponent.Deactivate` (`self.WingThrusterR`))
  (`ActorComponent.Deactivate` (`self.MainThruster`)))

(event `Multi_UpdateDamage`
  ;[1 0.54 0.54] Update damage particles
  (if (not (`KismetSystemLibrary.IsDedicatedServer`))
    (`self.UpdateDamageEffect`)))

(event `DestroySelf`
  (bind _returnvalue (`self.K2_GetActorLocation`))
  (bind _deathanim (`self.DeathAnim`))
  ;[0 0 0] Death Behavior
  (bind (_outhit _returnvalue_2) (`KismetSystemLibrary.LineTraceSingle` _returnvalue (- _returnvalue (0.0 0.0 250.0)) "ECC_GameTraceChannel11"))
  (if _returnvalue_2
    (`PrimalBuff.StaticAddBuff` "/Game/PrimalEarth/CoreBlueprints/Buffs/Buff_EndBossMorph_Dissolve_Out_Minion.Buff_EndBossMorph_Dissolve_Out_Minion_C" self null self)
    (if (`self.IsMontagePlaying` _deathanim)
      (`self.StopAnimEx` _deathanim false false 0.25))
    (else
      (`KismetSystemLibrary.K2_SetTimer` null "DestroySelf" 0.1))))

(event `self.BPTimerNonDedicated`
  (bind _returnvalue (`GameplayStatics.GetWorldDeltaSeconds`))
  ;[0.2384 0.8265 1] Update visuals (roll/pitch and turns)
  (`parent.BPTimerNonDedicated`)
  (if (`self.BPIsConscious`) :!label _label
    (`|ExecutionSequence`
      (:`then_0`
        (`self.UpdateAccel` _returnvalue))
      (:`then_1`
        (`self.Update Turn Anims And Rate` _returnvalue))
      (:`then_2`
        (`self.Update Visual Roll and Pitch` _returnvalue)))))

(event `ServerUpdateVisuals`
  ;[0.2384 0.8265 1] Update visuals (roll/pitch and turns)
  (goto _label))

(event `MC_Deactivate`
  (`/Engine/EditorBlueprintResources/ActorMacros.SwitchNetAuthority`
    (:`DedicatedServer`
      (`self.BPNetSetCharacterMovementVelocity` false (0.0 0.0 0.0) true "MOVE_Falling" :!label _label_2)
      (`self.ROS_Quit`))
    (:`PlayerServer`
      (`|ExecutionSequence`
        (:`then_0`
          (goto _label_2))
        (:`then_1`
          (`self.DeactivateDrone` :!label _label_3))))
    (:`Client`
      (goto _label_3))))

(event `MC_Activate`
  (`/Engine/EditorBlueprintResources/ActorMacros.SwitchNetAuthority`
    (:`DedicatedServer`
      (`self.BPNetSetCharacterMovementVelocity` false (0.0 0.0 0.0) true "MOVE_Flying" :!label _label_4))
    (:`PlayerServer`
      (`|ExecutionSequence`
        (:`then_0`
          (goto _label_4))
        (:`then_1`
          (`self.ActivateDrone` :!label _label_5))))
    (:`Client`
      (goto _label_5))))

(event `ROS_Quit`
  (bind _returnvalue (`self.GetCharacterController`))
  (bind _playerpawn (`self.PlayerPawn`))
  (`self.ROC_DisableInput`)
  (`/Engine/EditorBlueprintResources/StandardMacros.IsValid` _returnvalue
    (:`Is Valid`
      (`/Engine/EditorBlueprintResources/StandardMacros.IsValid` _playerpawn
        (:`Is Valid`
          (`Controller.Possess` _returnvalue _playerpawn)
          (set `self.PlayerPawn` null))))))

(event `Key|Q`
  (:`Pressed`
    (`self.ROS_Quit`)))

(event `ROC_EnableInput`
  (bind _returnvalue (`self.GetCharacterController`))
  (`/Engine/EditorBlueprintResources/StandardMacros.IsValid` _returnvalue
    (:`Is Valid`
      (bind _asshooterplayercontroller (cast `ShooterPlayerController` _returnvalue))
      (`self.EnableInput` _asshooterplayercontroller))))

(event `ROC_DisableInput`
  (bind _returnvalue (`self.GetCharacterController`))
  (`/Engine/EditorBlueprintResources/StandardMacros.IsValid` _returnvalue
    (:`Is Valid`
      (bind _asshooterplayercontroller (cast `ShooterPlayerController` _returnvalue))
      (`self.DisableInput` _asshooterplayercontroller))))

(fn `ActivateDrone`
  (bind _mesh (`self.Mesh`))
  (`ActorComponent.Activate` (`self.DamageEffect`) true)
  (`ActorComponent.Activate` (`self.MainThruster`) true)
  (`ActorComponent.Activate` (`self.WingThrusterR`) true)
  (`ActorComponent.Activate` (`self.WingThrusterL`) true)
  (`AudioComponent.FadeIn` (`self.Fly SFX`) 1.5 1.0 0.0)
  (if (> (`KismetArrayLibrary.Array_Length` (`MeshComponent.Materials` _mesh)) 0)
    (bind _returnvalue (`KismetMaterialLibrary.CreateDynamicMaterialInstance` "/Game/Mods/SamSpyDrone_Tut/SpyDrone/SpyDrone_Active_MIC.SpyDrone_Active_MIC"))
    (`PrimitiveComponent.SetMaterial` _mesh 0 _returnvalue)))

(fn `BPAdjustDamage`
  (params (IncomingDamage :type "Float (double-precision)") (TheDamageEvent :type "EngineTypes.DamageEvent Structure") (EventInstigator :type "Controller Object Reference") (DamageCauser :type "Actor Object Reference") (bIsPointDamage :type Boolean) (PointHitInfo :type "EngineTypes.HitResult Structure"))
  (returns (ReturnValue :type "Float (double-precision)"))
  (`|ExecutionSequence`
    (:`then_0`
      (if (not (`self.IsDead`))
        (`self.Multi_UpdateDamage`)))
    (:`then_1`
      (return IncomingDamage))))

(fn `DeactivateDrone`
  (bind _mesh (`self.Mesh`))
  (`ActorComponent.Deactivate` (`self.DamageEffect`))
  (`ActorComponent.Deactivate` (`self.MainThruster`))
  (`ActorComponent.Deactivate` (`self.WingThrusterR`))
  (`ActorComponent.Deactivate` (`self.WingThrusterL`))
  (`AudioComponent.FadeOut` (`self.Fly SFX`) 1.5 0.0)
  (if (> (`KismetArrayLibrary.Array_Length` (`MeshComponent.Materials` _mesh)) 0)
    (bind _returnvalue (`KismetMaterialLibrary.CreateDynamicMaterialInstance` "/Game/Mods/SamSpyDrone_Tut/SpyDrone/SpyDrone_InActive_MIC.SpyDrone_InActive_MIC"))
    (`PrimitiveComponent.SetMaterial` _mesh 0 _returnvalue)))

(fn `Update Turn Anims And Rate`
  (params (DeltaTime :type "Float (double-precision)"))
  (`|ExecutionSequence`
    (:`then_0`
      (bind (_rootrotoffset _therootyawspeed) (`self.GetAimOffsets` DeltaTime))
      (set `self.CurrentTurnRate` _therootyawspeed)
      (`|ExecutionSequence`
        (:`then_0`
          (bind _returnvalue (< _therootyawspeed -12.5))
          (if (and (not (`self.IsMontagePlaying` "/Game/EndGame/Dinos/Drone/Animations/Drone-Hover-Aim-Lft_Montage.Drone-Hover-Aim-Lft_Montage" 0.4)) _returnvalue)
            (`self.PlayAnimEx` "/Game/EndGame/Dinos/Drone/Animations/Drone-Hover-Aim-Lft_Montage.Drone-Hover-Aim-Lft_Montage")
            (set `self.RotorsRight` true)
            (elif (and (not _returnvalue) (`self.RotorsRight`))
              (`self.StopAnimEx` "/Game/EndGame/Dinos/Drone/Animations/Drone-Hover-Aim-Lft_Montage.Drone-Hover-Aim-Lft_Montage" false false 0.4)
              (set `self.RotorsRight` false))))
        (:`then_1`
          (bind _returnvalue_2 (> _therootyawspeed 12.5))
          (if (and _returnvalue_2 (not (`self.IsMontagePlaying` "/Game/EndGame/Dinos/Drone/Animations/Drone-Hover-Aim-Rit_Montage.Drone-Hover-Aim-Rit_Montage" 0.4)))
            (`self.PlayAnimEx` "/Game/EndGame/Dinos/Drone/Animations/Drone-Hover-Aim-Rit_Montage.Drone-Hover-Aim-Rit_Montage")
            (set `self.RotorsLeft` true)
            (elif (and (not _returnvalue_2) (`self.RotorsLeft`))
              (`self.StopAnimEx` "/Game/EndGame/Dinos/Drone/Animations/Drone-Hover-Aim-Rit_Montage.Drone-Hover-Aim-Rit_Montage" false false 0.4)
              (set `self.RotorsLeft` false))))))
    (:`then_1`
      (return))))

(fn `Update Visual Roll and Pitch`
  (params (DeltaTime :type "Float (double-precision)"))
  (bind _returnvalue (`self.GetVelocity` false))
  (bind _returnvalue_2 (`KismetMathLibrary.Dot_VectorVector` _returnvalue (`self.GetActorForwardVector`)))
  (bind _returnvalue_3 (`KismetMathLibrary.Dot_VectorVector` _returnvalue (`self.GetActorRightVector`)))
  (bind _yaw (.yaw (`CharacterMovementComponent.RotationRate` (`self.CharacterMovement`))))
  (bind _returnvalue_4 (* (`CharacterMovementComponent.MaxFlySpeed` (`self.CharacterMovement`)) (`self.FlyingRunSpeedModifier`) (`self.RunningSpeedModifier`)))
  (bind _returnvalue_5 (`KismetMathLibrary.SelectFloat` 1e-05 _returnvalue_4 (== _returnvalue_4 0.0)))
  (`SceneComponent.SetRelativeRotation` (`self.Mesh`) (`KismetMathLibrary.MakeRot` (`KismetMathLibrary.SelectFloat` (`KismetMathLibrary.FInterpTo` (.pitch (`SceneComponent.RelativeRotation` (`self.Mesh`))) (`KismetMathLibrary.FClamp` (+ (`KismetMathLibrary.SelectFloat` (* 20.0 (/ _returnvalue_3 _returnvalue_5)) 0.0 (>= (`KismetMathLibrary.Abs` _returnvalue_3) 50.0)) (* (/ (`self.CurrentTurnRate`) (`KismetMathLibrary.SelectFloat` 1e-05 _yaw (== _yaw 0.0))) 20.0)) -35.0 35.0) DeltaTime 3.0) 0.0 (`self.UseInterpRoll`)) -90.0 (`KismetMathLibrary.SelectFloat` (`KismetMathLibrary.FInterpTo` (.roll (`SceneComponent.RelativeRotation` (`self.Mesh`))) (`KismetMathLibrary.SelectFloat` (* 10.0 (/ _returnvalue_2 _returnvalue_5)) 0.0 (>= (`KismetMathLibrary.Abs` _returnvalue_2) 50.0)) DeltaTime 2.0) 0.0 (`self.UseInterpPitch`))) false)
  (return))

(fn `UpdateAccel`
  (params (DeltaTime :type "Float (double-precision)"))
  (bind _returnvalue (`KismetMathLibrary.SelectFloat` 1e-05 DeltaTime (== DeltaTime 0.0)))
  (bind _velocity (`MovementComponent.Velocity` (`self.CharacterMovement`)))
  (set `self.CurrentAcceleration` (/ (`KismetMathLibrary.VInterpTo_Constant` (`self.LastVelocity`) _velocity _returnvalue 10.0) _returnvalue))
  (set `self.LastVelocity` _velocity))

(fn `UpdateDamageEffect`
  (`ParticleSystemComponent.SetFloatParameter` (`self.DamageEffect`) "Damage - Amount" (- 1.0 (`self.GetHealthPercentage`))))

(fn `UserConstructionScript`
  (`parent.UserConstructionScript`))